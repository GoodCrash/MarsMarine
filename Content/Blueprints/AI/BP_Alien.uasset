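; BP_Alien is an enemy character that chases and melee-attacks the player until killed.
; A looping AI MoveTo drives pursuit, while Tick pauses movement to play an attack montage when in range.
; DamagePlayer applies hit damage but is not called within these graphs.
; Damage lowers health, and a hit arriving at zero health triggers death, crediting BP_Marine's kills, notifying BP_GameMode, and destroying the actor after a delay.
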(event `self.ReceiveBeginPlay`
  ;[1 1 1] Alien to Chase Player
  (if (`self.IsAlive`) :!label _label
    (`|AIMoveTo` self (0.0 0.0 0.0) (`GameplayStatics.GetPlayerCharacter` 0)
      (:`OnSuccess`
        _)
      (:`OnFail`
        _))
    (`KismetSystemLibrary.Delay` 0.2)
    (goto _label)))

(event `self.ReceiveTick`
  (params (DeltaSeconds :type "Float (single-precision)"))
  ;[1 1 1] Alien Attack
  (if (`self.CanAttack`)
    (`self.DeactivateAIMovement`)
    (`|PlayMontage` (`self.Mesh`) "/Game/Characters/Enemy_Great_Spider/Animations/AlienAttack1.AlienAttack1"
      (:`OnCompleted`
        (`self.ActivateAIMovement`)))))

(event `self.ReceiveAnyDamage`
  (params (Damage :type "Float (single-precision)") (DamageType :type "DamageType Object Reference") (InstigatedBy :type "Controller Object Reference") (DamageCauser :type "Actor Object Reference"))
  ;[1 1 1] Alien Get Domage and Dieing
  (if (> (`self.Health`) 0.0)
    (`self.DecreaseHealth` Damage)
    (else
      (`self.DyingAIein`)
      (`KismetSystemLibrary.Delay` 3.0)
      (`self.K2_DestroyActor`))))

(fn `ActivateAIMovement`
  (`ActorComponent.Activate` (`self.CharacterMovement`) false))

(fn `CanAttack`
  (returns (ReturnValue :type Boolean))
  (return (and (`self.IsAlive`) (`self.IsWithinAttackRange`) (not (`self.IsAttacking`)))))

(fn `DamagePlayer`
  (`GameplayStatics.ApplyDamage` (`GameplayStatics.GetPlayerCharacter` 0) (`self.DamagePerHit`)))

(fn `DeactivateAIMovement`
  (bind _charactermovement (`self.CharacterMovement`))
  (`MovementComponent.StopMovementImmediately` _charactermovement)
  (`ActorComponent.Deactivate` _charactermovement))

(fn `DecreaseHealth`
  (params (DamageAmount :type "Float (double-precision)"))
  (set `self.Health` (`KismetMathLibrary.FClamp` (- (`self.Health`) DamageAmount) 0.0 100.0)))

(fn `DyingAIein`
  (set `self.IsDead` true)
  (`self.DeactivateAIMovement`)
  (`self.SetActorEnableCollision` false)
  (bind _asbp_marine (cast `/Game/Blueprints/Pawns/BP_Marine` (`GameplayStatics.GetPlayerCharacter` 0)))
  (`/Game/Blueprints/Pawns/BP_Marine.IncreaseKills` _asbp_marine)
  (bind _asbp_game_mode (cast `/Game/Blueprints/GameMode/BP_GameMode` (`GameplayStatics.GetGameMode`)))
  (`/Game/Blueprints/GameMode/BP_GameMode.RegisterAlienDeath` _asbp_game_mode self))

(fn `IsAlive`
  (returns (NotDead :type Boolean))
  (return (not (`self.IsDead`))))

(fn `IsAttacking`
  (returns (NewParam :type Boolean))
  (return (`AnimInstance.Montage_IsPlaying` (`SkeletalMeshComponent.GetAnimInstance` (`self.Mesh`)) "/Game/Characters/Enemy_Great_Spider/Animations/AlienAttack1.AlienAttack1")))

(fn `IsWithinAttackRange`
  (returns (NewParam :type Boolean))
  (return (< (`self.GetDistanceTo` (`GameplayStatics.GetPlayerCharacter` 0)) (`self.AttackRange`))))

(fn `UserConstructionScript`)